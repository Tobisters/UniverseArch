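; BP_DrumKeyboard is a VR drum-style virtual keyboard that edits the text of the entity selected on BP_Globe.
; It binds every child BP_DrumButton's press event, then appends text behind a trailing underscore cursor or handles modifier keys.
; A history array drives backspace, a character limit caps input, and WidgetInteraction forwards keys.
; Enter commits the text, destroys the keyboard, hides both mallets and re-enables spawning and flying.
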(event `self.ReceiveBeginPlay`
  ;[1 1 1] // Button Setup
  (`|ExecutionSequence`
    (:`then_0`
      (bind _output_get (set `self.KeyboardButtons` (`self.K2_GetComponentsByClass` "/Script/Engine.ChildActorComponent")))
      ;;[1 1 1] // Bind 'Button Pressed' dispatcher event to each button being used
      (for _array_element _output_get
        (bind _asbp_drum_button (cast `/Game/VRKeyboards/Blueprints/Keyboards/Drum/BP_DrumButton` (`ChildActorComponent.ChildActor` _array_element)))
        (add `/Game/VRKeyboards/Blueprints/Keyboards/Drum/BP_DrumButton.Button pressed` _asbp_drum_button (delegate `ButtonPressed`))))
    (:`then_1`
      ;;[1 1 1] Get Globe reference (used to print the string from the keyboard)
      (bind _outactors (`GameplayStatics.GetAllActorsOfClass` "/Game/VirtualRealityBP/Blueprints/BP_Globe.BP_Globe_C"))
      (set `self.Globe` (`|GetArrayItem` _outactors)))))

(event `ButtonPressed`
  (params (ButtonText :type Text) (Modifier :type "/Game/VRKeyboards/Blueprints/Enums/EModifierKeys Enum" :default "NewEnumerator2"))
  ;[1 1 1] // Button Setup
  ;;[1 1 1] // Bind 'Button Pressed' dispatcher event to each button being used
  (`self.DrumKeyboardButtonPressed` ButtonText Modifier))

(event `DrumKeyboardButtonPressed`
  (params (TextToUse :type Text) (ModifierKey :type "/Game/VRKeyboards/Blueprints/Enums/EModifierKeys Enum" :default "NewEnumerator2"))
  ;[1 1 1] // Button Setup
  ;;[1 1 1] // Keyboard Button Pressed Event
  ;; // If a Keyboard Button is pressed, then perform it's given purpose.
  (`self.DetermineButtonFunctionality` TextToUse ModifierKey))

(fn `AddTextToMessageBox`
  (params (ButtonTextToUse :type Text))
  (bind _text (`TextRenderComponent.Text` (`/Game/VirtualRealityBP/Blueprints/BP_Globe.TextRendererOfSelectedEntity` (`self.Globe`))))
  (bind _returnvalue (`KismetTextLibrary.Conv_StringToText` (`KismetStringLibrary.Concat_StrStr` (`KismetStringLibrary.Split` (`KismetTextLibrary.Conv_TextToString` _text) "_" "IgnoreCase" "FromEnd") (`KismetTextLibrary.Conv_TextToString` ButtonTextToUse) "_")))
  (if (not (== (`self.CurrentNumOfCharacters`) (`self.CharacterLimit`)))
    (set `self.CurrentNumOfCharacters` (+ (`self.CurrentNumOfCharacters`) 1))
    (`KismetArrayLibrary.Array_Add` (`self.PreviouslyAddedText`) _text)
    (`TextRenderComponent.K2_SetText` (`self.MessageBoxText`) _returnvalue)
    (`TextRenderComponent.K2_SetText` (`/Game/VirtualRealityBP/Blueprints/BP_Globe.TextRendererOfSelectedEntity` (`self.Globe`)) _returnvalue)
    (`self.SendText` _returnvalue)))

(fn `ClearMessageBox`
  (`TextRenderComponent.K2_SetText` (`self.MessageBoxText`) "_")
  (`TextRenderComponent.K2_SetText` (`/Game/VirtualRealityBP/Blueprints/BP_Globe.TextRendererOfSelectedEntity` (`self.Globe`)) "_"))

(fn `DetermineButtonFunctionality`
  (params (ButtonText :type Text) (ModifierKey :type "/Game/VRKeyboards/Blueprints/Enums/EModifierKeys Enum" :default "NewEnumerator2"))
  (locals (ModifierToCheck :type "/Game/VRKeyboards/Blueprints/Enums/EModifierKeys Enum") (TextToUse :type Text))
  (set `local.TextToUse` ButtonText)
  (bind _output_get (set `local.ModifierToCheck` ModifierKey))
  ;[1 1 1] // Is a modifier key being used?
  ; // NOTE: 'None' means the key is NOT a modifier key.
  (if (`|EnumEquality` _output_get "NewEnumerator2")
    (`self.AddTextToMessageBox` (`local.TextToUse`))
    (else
      (`self.UseModifierKey` (`local.ModifierToCheck`)))))

(fn `RemoveTextFromMessageBox`
  (bind _previouslyaddedtext (`self.PreviouslyAddedText`))
  (bind _returnvalue (`KismetArrayLibrary.Array_Length` _previouslyaddedtext))
  (bind _returnvalue_2 (- _returnvalue 1))
  (bind _output (`|GetArrayItem` _previouslyaddedtext _returnvalue_2))
  (if (== _returnvalue 0)
    (return)
    (else
      (`TextRenderComponent.K2_SetText` (`self.MessageBoxText`) _output)
      (`TextRenderComponent.K2_SetText` (`/Game/VirtualRealityBP/Blueprints/BP_Globe.TextRendererOfSelectedEntity` (`self.Globe`)) _output)
      (`KismetArrayLibrary.Array_Remove` (`self.PreviouslyAddedText`) _returnvalue_2)
      (set `self.CurrentNumOfCharacters` (- (`self.CurrentNumOfCharacters`) 1))
      (return))))

(fn `SendText`
  (params (TextToSend :type "Text (by ref)"))
  (`WidgetInteractionComponent.SendKeyChar` (`self.WidgetInteraction`) (`KismetTextLibrary.Conv_TextToString` TextToSend) false))

(fn `UseModifierKey`
  (params (Modifier :type "/Game/VRKeyboards/Blueprints/Enums/EModifierKeys Enum" :default "NewEnumerator2"))
  (bind _globe (`self.Globe`))
  (bind _textrendererofselectedentity (`/Game/VirtualRealityBP/Blueprints/BP_Globe.TextRendererOfSelectedEntity` (`self.Globe`)))
  (bind _textrendererofselectedentity2 (`/Game/VirtualRealityBP/Blueprints/BP_Globe.TextRendererOfSelectedEntity2` _globe))
  (bind _returnvalue (`KismetTextLibrary.Conv_StringToText` (`KismetStringLibrary.Split` (`KismetTextLibrary.Conv_TextToString` (`TextRenderComponent.Text` _textrendererofselectedentity)) "_")))
  (switch `/Game/VRKeyboards/Blueprints/Enums/EModifierKeys` Modifier
    (:`NewEnumerator0`
      (`self.AddTextToMessageBox` " ")
      (`WidgetInteractionComponent.PressAndReleaseKey` (`self.WidgetInteraction`) "SpaceBar"))
    (:`NewEnumerator1`
      (`self.RemoveTextFromMessageBox`)
      (`WidgetInteractionComponent.PressAndReleaseKey` (`self.WidgetInteraction`) "BackSpace"))
    (:`NewEnumerator6`
      (`self.EnterButtonPressed`)
      (`TextRenderComponent.K2_SetText` _textrendererofselectedentity _returnvalue)
      (`/Engine/EditorBlueprintResources/StandardMacros.IsValid` _textrendererofselectedentity2
        (:`Is Valid`
          (`TextRenderComponent.K2_SetText` _textrendererofselectedentity2 _returnvalue)
          (set `/Game/VirtualRealityBP/Blueprints/BP_Globe.TextRendererOfSelectedEntity2` null _globe))
        (:`Is Not Valid`
          _))
      ;[1 1 1] Destroy keyboard and mallots
      (`self.K2_DestroyActor`)
      (bind _asfly_player (cast `/Game/Character/FlyPlayer` (`GameplayStatics.GetPlayerCharacter` 0)))
      (`SceneComponent.SetVisibility` (`/Game/VirtualRealityBP/Blueprints/BP_MotionController.DrumMallot` (`/Game/Character/FlyPlayer.LeftController` _asfly_player)) false false)
      (`SceneComponent.SetVisibility` (`/Game/VirtualRealityBP/Blueprints/BP_MotionController.DrumMallot` (`/Game/Character/FlyPlayer.RightController` _asfly_player)) false false)
      (`/Game/VirtualRealityBP/Blueprints/BP_Globe.Allow Spawning` (`self.Globe`))
      (set `/Game/Character/FlyPlayer.AllowFlying` true _asfly_player))
    (:`NewEnumerator3`
      (for _array_element (`self.KeyboardButtons`)
        (message `/Game/VRKeyboards/Blueprints/Interfaces/BPI_KeyboardInteraction.CapsLock` (`ChildActorComponent.ChildActor` _array_element))))
    (:`NewEnumerator4`
      (for _array_element_2 (`self.KeyboardButtons`)
        (message `/Game/VRKeyboards/Blueprints/Interfaces/BPI_KeyboardInteraction.SymbolLock` (`ChildActorComponent.ChildActor` _array_element_2))))
    (:`NewEnumerator5`
      (`self.WebBrowserButtonPressed`))))

(fn `UserConstructionScript`)