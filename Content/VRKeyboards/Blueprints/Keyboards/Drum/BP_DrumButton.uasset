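; BP_DrumButton is a single key of a VR drum-style keyboard, struck with a BP_DrumMallot.
; A mallet overlap passes a DoOnce, plays a sound and runs a timeline that moves the key on Z.
; When the forward stroke ends, it reverses, re-arms and broadcasts ButtonPressed with its text and modifier for BP_DrumKeyboard.
; CapsLock and SymbolLock events toggle the label, while construction applies optional mesh, material and scale overrides.
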(event `self.ReceiveBeginPlay`
  ;[1 1 1] // Event Begin Play
  ; // Set the button's text to it's UpperCase text
  (`self.SetButtonText` (`self.UpperCaseText`)))

(event `/Game/VRKeyboards/Blueprints/Interfaces/BPI_KeyboardInteraction.CapsLock`
  ;[1 1 1] // Caps Lock
  ; // Switches the button text to an upper or lowercase letter
  (`self.ChangeButtonTextCasing`))

(event `/Game/VRKeyboards/Blueprints/Interfaces/BPI_KeyboardInteraction.SymbolLock`
  ;[1 1 1] // Switches the button text to a symbol (Special Text)
  (`self.ChangeButtonTextToSymbols`))

(event `self.Button.OnComponentBeginOverlap`
  (params (OverlappedComponent :type "PrimitiveComponent Object Reference") (OtherActor :type "Actor Object Reference") (OtherComp :type "PrimitiveComponent Object Reference") (OtherBodyIndex :type Integer) (bFromSweep :type Boolean) (SweepResult :type "HitResult Structure (by ref)"))
  ;[1 1 1] // Button movement when pressed
  ;;[0 0.56 0.01732] // This is what controls triggering the button movement
  (cast `/Game/VRKeyboards/Blueprints/Keyboards/Drum/BP_DrumMallot` OtherActor)
  (`/Engine/EditorBlueprintResources/StandardMacros.DoOnce` false :!label _label
    (:`Completed`
      (`GameplayStatics.PlaySound2D` (`self.ButtonSFX`) 1.0 1.0 0.0 null null)
      (bind (_direction _press) (`Timeline|Press` :!via `PlayFromStart` :!label _label_2) ; Timeline for animating the button press
        (:`Update`
          (`SceneComponent.K2_SetRelativeLocation` (`self.Button`) (`KismetMathLibrary.MakeVector` 0.0 0.0 _press) false true) ; Move button up/down
        )
        (:`Finished`
          (if (`|EnumEquality` _direction "Forward")
            (`self.ReverseButton`)
            ;[1 1 1] // Button Pressed (dispatcher event)
            ;
            ; // After the button has been pressed and released, the button's function will be sent to all subscribers of the dispatcher event (which in this case will be BP_DrumKeyboard).
            (`self.Button pressed` (`TextRenderComponent.Text` (`self.ButtonText`)) (`self.Modifier`))))))))

(event `ReverseButton`
  ;[1 1 1] // Button movement when pressed
  (`|ExecutionSequence`
    (:`then_0`
      (goto _label_2 :!via `ReverseFromEnd`))
    (:`then_1`
      (goto _label :!via `Reset`))))

(fn `ChangeButtonTextCasing`
  ;[1 1 1] // If the Current Text is Uppercase then switch to Lowercase. Likewise, if Lowercase then switch to Uppercase.
  (if (`KismetTextLibrary.EqualEqual_TextText` (`TextRenderComponent.Text` (`self.ButtonText`)) (`self.UpperCaseText`))
    (set `self.CurrentText` (`self.LowerCaseText`))
    (else
      (set `self.CurrentText` (`self.UpperCaseText`))))
  (`self.SetButtonText` (`self.CurrentText`))
  (return))

(fn `ChangeButtonTextToSymbols`
  (`self.SetButtonText` (select `bool` (== (`TextRenderComponent.Text` (`self.ButtonText`)) (`self.SecondaryText`)) :`false` (`self.SecondaryText`) :`true` (`self.UppercaseText`)))
  (return))

(fn `SetButtonText`
  (params (TextToSetTo :type "Text (by ref)"))
  (`TextRenderComponent.K2_SetText` (`self.ButtonText`) TextToSetTo))

(fn `UserConstructionScript`
  (bind _buttonmaterial (`self.ButtonMaterial`))
  ;[1 1 1] // Change default button material if a new one was selected in BP_DrumKeyboard.
  (`/Engine/EditorBlueprintResources/StandardMacros.IsValid` _buttonmaterial
    (:`Is Valid`
      (`PrimitiveComponent.SetMaterial` (`self.Button`) 0 _buttonmaterial))
    (:`Is Not Valid`
      _))
  ;[1 1 1] // Change the default button mesh if a new one was selected in BP_DrumKeyboard.
  (`/Engine/EditorBlueprintResources/StandardMacros.IsValid` (`self.ButtonMesh`)
    (:`Is Valid`
      (`StaticMeshComponent.SetStaticMesh` (`self.Button`) (`self.ButtonMesh`))
      ;[1 1 1] // Set the button's new relative scale if a new one was set in BP_DrumKeyboard.
      (`SceneComponent.SetRelativeScale3D` (`self.Button`) (`self.RelativeScale`)))))